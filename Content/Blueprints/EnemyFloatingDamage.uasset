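; Floating damage text actor for enemies, showing a value passed to SetText on a recolored TextRender.
; BeginPlay builds a movement vector from the axis speeds, randomly flipping the Y direction so the text drifts to either side.
; Each Tick offsets the actor by that vector, then FloatMotion steadily reduces X speed to arc the motion along X.
; Movement is per frame, with no delta-time scaling.
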(event EventBeginPlay
  (if (== (Math|Random|RandomIntegerinRange 0 1) 0)
    (Variables|Default|SetAxis -1)
    (else
      (Variables|Default|SetAxis 1)))
  (Variables|Default|SetTextMovementVector (Math|Vector|MakeVector (Variables|Default|GetX_Speed) (* (Variables|Default|GetAxis) (Variables|Default|GetY_Speed)) (Variables|Default|GetZ_Speed))))

(event Collision|EventActorBeginOverlap
  (params (OtherActor :type Actor%20Object%20Reference)))

(event EventTick
  (params (DeltaSeconds :type Float%20%28single-precision%29))
  (Transformation|SetActorLocation (+ (Transformation|GetActorLocation self) (Variables|Default|GetTextMovementVector)) false false)
  (CallFunction|FloatMotion))

(fn ConstructionScript)

(fn SetText
  (params (Text :type Text))
  (bind _textrender (Variables|Default|GetTextRender))
  (Rendering|Components|TextRender|SetText _textrender Text)
  (Rendering|Components|TextRender|SetTextRenderColor _textrender (Math|Color|MakeColor 255 0 0)))

(fn FloatMotion
  (Variables|Default|SetTextMovementVector (Math|Vector|MakeVector (Variables|Default|GetX_Speed) (.Y (Math|Vector|BreakVector (Variables|Default|GetTextMovementVector))) (.Z (Math|Vector|BreakVector (Variables|Default|GetTextMovementVector)))))
  (Variables|Default|SetX_Speed (- (Variables|Default|GetX_Speed) (Variables|Default|GetTextDropSpeed)))
  (return))