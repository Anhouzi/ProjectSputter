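; Behavior Tree task that sends an AI-controlled Mook toward a lead point ahead of its TargetToFollow, a TwinStickPawn.
; LeadLocation offsets the target's position by its velocity times a multiplier, which is raised at high GameDifficulty.
; Once AIMoveTo is issued, it sets walk speed by distance to the target, zero when close, and finishes without waiting for arrival.
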(event EventReceiveExecute
  (params (OwnerActor :type Actor%20Object%20Reference))
  (if (!= (Variables|Default|GetAI_ControllerRef) 0)
    _
    (else
      (bind _asai_controller (Utilities|Casting|CastToAI_Controller OwnerActor))
      (Variables|Default|SetAI_ControllerRef _asai_controller)))
  (bind _leadvector (CallFunction|LeadLocation))
  (AI|AIMoveTo (Pawn|GetControlledPawn (Variables|Default|GetAI_ControllerRef)) _leadvector 0 5e+01 false
    (:then
      (if (!= (Pawn|GetControlledPawn (Variables|Default|GetAI_ControllerRef)) 0)
        (bind _asmook (Utilities|Casting|CastToMook (Pawn|GetControlledPawn (Variables|Default|GetAI_ControllerRef))))
        (bind _output_get (Variables|Default|SetCharacterMoveRef (Variables|/Script/Engine.Character|GetCharacterMovement _asmook)))
        (if (>= (Math|Vector|VectorLength (- (Transformation|GetActorLocation (Pawn|GetControlledPawn (Variables|Default|GetAI_ControllerRef))) (Transformation|GetActorLocation (AI|BehaviorTree|GetBlackboardValueasActor (Variables|Default|GetTargetToFollow))))) 4e+02)
          (Variables|/Script/Engine.CharacterMovementComponent|SetMaxWalkSpeed _output_get 3e+02)
          (else
            (Variables|/Script/Engine.CharacterMovementComponent|SetMaxWalkSpeed _output_get 0.0)))
        (AI|BehaviorTree|FinishExecute true)))))

(fn LeadLocation
  (bind _targettofollow (Variables|Default|GetTargetToFollow))
  (bind _returnvalue (AI|BehaviorTree|GetBlackboardValueasActor _targettofollow))
  (bind _asmy_game_instance (Utilities|Casting|CastToMyGameInstance (Game|GetGameInstance)))
  (bind _astwin_stick_pawn (Utilities|Casting|CastToTwinStickPawn _returnvalue))
  (if (>= (Variables|/Game/Levels/MyGameInstance.MyGameInstance_C|GetGameDifficulty _asmy_game_instance) 5)
    (LocalVariables|SetLeadMultiplier 10))
  (return (+ (Transformation|GetActorLocation _returnvalue) (* (Variables|/Game/TwinStickBP/Blueprints/TwinStickPawn.TwinStickPawn_C|GetVelocityVector _astwin_stick_pawn) (LocalVariables|GetLeadMultiplier)))))