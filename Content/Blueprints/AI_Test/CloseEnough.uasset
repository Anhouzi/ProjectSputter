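; CloseEnough is a behavior tree decorator condition that checks whether an AI's pawn is within aggro range of its follow target.
; It casts the owner to AI_Controller, stores that reference, and reads the target actor from the TargetToFollow blackboard key.
; The check passes when the straight-line distance between the controlled pawn and that actor is at most AggroRange.
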(fn PerformConditionCheck
  (params (OwnerActor :type Actor%20Object%20Reference))
  (bind _asai_controller (Utilities|Casting|CastToAI_Controller OwnerActor))
  (Variables|Default|SetAI_ControllerRef _asai_controller)
  (return (<= (Math|Vector|VectorLength (- (Transformation|GetActorLocation (Pawn|GetControlledPawn (Variables|Default|GetAI_ControllerRef))) (Transformation|GetActorLocation (AI|BehaviorTree|GetBlackboardValueasActor (Variables|Default|GetTargetToFollow))))) (Variables|Default|GetAggroRange))))