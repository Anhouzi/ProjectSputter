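; AI controller that sets up blackboard and behavior tree for the pawn it controls.
; On BeginPlay it uses MyBlackBoard, waits briefly, then stores the pawn's current location as the HomeLocation key.
; It runs BT_Mook2 when the pawn casts to Mook, and MyBehaviorTree for any other pawn.
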(event EventBeginPlay
  (Class|AIController|UseBlackboard "/Game/Blueprints/AI_Test/MyBlackBoard.MyBlackBoard")
  (Utilities|FlowControl|Delay 0.1)
  ;[1 1 1] Setting home location for the actor.
  (AI|Components|Blackboard|SetValueasVector (AI|GetBlackboard self) (Variables|Default|GetHomeLocation) (Transformation|GetActorLocation (Pawn|GetControlledPawn)))
  (Utilities|Casting|CastToMook (Pawn|GetControlledPawn)
    (:then
      (AI|RunBehaviorTree "/Game/Enemies/Mook/Blueprints/BT_Mook2.BT_Mook2"))
    (:CastFailed
      (AI|RunBehaviorTree "/Game/Blueprints/AI_Test/MyBehaviorTree.MyBehaviorTree"))))

(fn ConstructionScript)