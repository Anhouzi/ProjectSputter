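; AI_Character is an enemy character for a twin-stick shooter that spawns its own AI controller and fires projectiles.
; Tick advances the weapon cooldown, or at zero health credits the player pawn with a kill and destroys the actor.
; Twin-stick projectile hits apply the player's damage scaled by DamageReduction and spawn floating damage text.
; EnemySetup scales health and weapon strength from a modifier, and FireWeapon spawns cooldown-gated projectiles carrying that strength.
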(event Collision|EventHit
  (params (MyComp :type Primitive%20Component%20Object%20Reference) (Other :type Actor%20Object%20Reference) (OtherComp :type Primitive%20Component%20Object%20Reference) (bSelfMoved :type Boolean) (HitLocation :type Vector :default "0, 0, 0") (HitNormal :type Vector :default "0, 0, 0") (NormalImpulse :type Vector :default "0, 0, 0") (Hit :type Hit%20Result%20Structure%20%28by%20ref%29))
  (bind _self self)
  (bind _returnvalue (Transformation|GetActorLocation _self))
  (bind (_x _y _z) (Math|Vector|BreakVector _returnvalue))
  (Utilities|Casting|CastToTwinStickProjectile Other)
  (bind _astwin_stick_pawn (Utilities|Casting|CastToTwinStickPawn (Game|Player|GetPlayerPawn 0)))
  (bind _returnvalue_2 (Game|SpawnActorfromClass "/Game/Blueprints/EnemyFloatingDamage.EnemyFloatingDamage_C" (Math|Transform|MakeTransform (Math|Vector|MakeVector _x _y (+ _z 5e+01)) "90.000000,180.000000,0.000000") "Undefined" 0 0))
  (bind _finaldamage (CallFunction|DamageCalculations (Variables|/Game/TwinStickBP/Blueprints/TwinStickPawn.TwinStickPawn_C|GetDamageValue _astwin_stick_pawn)))
  (Default|SetText _returnvalue_2 (Utilities|Text|ToText(Float) _finaldamage "HalfToEven")))

(event EventBeginPlay
  (Pawn|SpawnDefaultController))

(event EventTick
  (params (DeltaSeconds :type Float%20%28single-precision%29))
  (if (<= (Variables|Default|GetHealth) 0.0)
    (bind _astwin_stick_pawn (Utilities|Casting|CastToTwinStickPawn (Game|Player|GetPlayerPawn 0)))
    (Math|Integer|IncrementInt (Variables|/Game/TwinStickBP/Blueprints/TwinStickPawn.TwinStickPawn_C|GetNumberOfKills _astwin_stick_pawn)
      (:%20%20
        (Actor|DestroyActor)))
    (else
      (Variables|Default|SetWeaponCooldown (+ (Variables|Default|GetWeaponCooldown) DeltaSeconds)))))

(fn ConstructionScript)

(fn DamageCalculations
  (params (IncomingDamage :type Float%20%28single-precision%29))
  (bind _damagereduction (Variables|Default|GetDamageReduction))
  (bind _returnvalue (* IncomingDamage _damagereduction))
  (Variables|Default|SetHealth (- (Variables|Default|GetHealth) _returnvalue))
  (return _returnvalue))

(fn FireWeapon
  (bind _self self)
  (bind _weaponoffset (Variables|Default|GetWeaponOffset))
  (bind _returnvalue (Transformation|GetActorForwardVector _self))
  (bind (_x _y _z) (Math|Vector|BreakVector _returnvalue))
  (if (>= (Variables|Default|GetWeaponCooldown) (Variables|Default|GetWeaponSpeed))
    (bind _returnvalue_2 (Game|SpawnActorfromClass "/Game/TwinStickBP/Blueprints/GeneralProjectile.GeneralProjectile_C" (Math|Transform|MakeTransform (+ (Transformation|GetWorldLocation (Variables|Default|GetSphere)) (Math|Vector|MakeVector (* _x _weaponoffset) (* _y _weaponoffset) _z)) (Transformation|GetActorRotation) (Variables|Default|GetProjectileScale)) "AlwaysSpawn" 0 0))
    (Variables|/Game/TwinStickBP/Blueprints/GeneralProjectile.GeneralProjectile_C|SetDamageValue _returnvalue_2 (Variables|Default|GetWeaponStrength))
    (Variables|Default|SetWeaponCooldown 0.0)))

(fn EnemySetup
  (params (Modifier :type Float%20%28single-precision%29))
  (LocalVariables|SetEnemyModifier Modifier)
  (Variables|Default|SetHealth (+ (Variables|Default|GetHealth) (/ (LocalVariables|GetEnemyModifier) 2.0)))
  (Variables|Default|SetWeaponStrength (* (LocalVariables|GetEnemyModifier) 0.1)))