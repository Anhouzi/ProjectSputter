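; Mook is a twin-gun enemy for a twin-stick shooter that spawns its default controller on BeginPlay.
; Tick advances the weapon cooldown and checks health, destroying the actor and crediting the player's kill count at zero.
; Projectile hits apply the player pawn's damage value, scaled by DamageReduction, and spawn floating damage text.
; FireRightWeapon gates both guns' randomly spread shots on cooldown, while EnemySetup derives health and weapon strength from a modifier.
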(event Custom|IsDead?
  (if (<= (Variables|Default|GetHealth) 0.0)
    (Math|Integer|IncrementInt (Variables|/Game/TwinStickBP/Blueprints/TwinStickPawn.TwinStickPawn_C|GetNumberOfKills (Variables|Default|GetPlayerRef))
      (:%20%20
        (Actor|DestroyActor)))))

(event EventTick
  (params (DeltaSeconds :type Float%20%28single-precision%29))
  (CallFunction|IsDead?)
  (Variables|Default|SetWeaponCooldown (+ (Variables|Default|GetWeaponCooldown) DeltaSeconds)))

(event Collision|EventHit
  (params (MyComp :type Primitive%20Component%20Object%20Reference) (Other :type Actor%20Object%20Reference) (OtherComp :type Primitive%20Component%20Object%20Reference) (bSelfMoved :type Boolean) (HitLocation :type Vector :default "0, 0, 0") (HitNormal :type Vector :default "0, 0, 0") (NormalImpulse :type Vector :default "0, 0, 0") (Hit :type Hit%20Result%20Structure%20%28by%20ref%29))
  (bind _self self)
  (bind _returnvalue (Transformation|GetActorLocation _self))
  (bind (_x _y _z) (Math|Vector|BreakVector _returnvalue))
  (Utilities|Casting|CastToTwinStickProjectile Other)
  (bind _astwin_stick_pawn (Utilities|Casting|CastToTwinStickPawn (Game|Player|GetPlayerPawn 0)))
  (bind _returnvalue_2 (Game|SpawnActorfromClass "/Game/Blueprints/EnemyFloatingDamage.EnemyFloatingDamage_C" (Math|Transform|MakeTransform (Math|Vector|MakeVector _x _y (+ _z (Variables|Default|GetModelHeight))) "90.000000,180.000000,0.000000") "Undefined" 0 0))
  (bind _finaldamage (CallFunction|DamageCalculations (Variables|/Game/TwinStickBP/Blueprints/TwinStickPawn.TwinStickPawn_C|GetDamageValue _astwin_stick_pawn)))
  (Default|SetText _returnvalue_2 (Utilities|Text|ToText(Float) _finaldamage "HalfToEven")))

(event EventBeginPlay
  (bind _astwin_stick_pawn (Utilities|Casting|CastToTwinStickPawn (Pawn|GetControlledPawn (Game|GetPlayerController 0))))
  (Variables|Default|SetPlayerRef _astwin_stick_pawn)
  (Pawn|SpawnDefaultController))

(fn ConstructionScript)

(fn DamageCalculations
  (params (IncomingDamage :type Float%20%28single-precision%29))
  (bind _damagereduction (Variables|Default|GetDamageReduction))
  (bind _returnvalue (* IncomingDamage _damagereduction))
  (Variables|Default|SetHealth (- (Variables|Default|GetHealth) _returnvalue))
  (return _returnvalue))

(fn FireRightWeapon
  (bind _returnvalue (Transformation|GetActorRotation))
  (bind _self self)
  (bind _weaponoffset (Variables|Default|GetWeaponOffset))
  (bind _returnvalue_2 (Transformation|GetActorForwardVector _self))
  (bind (_roll _pitch _yaw) (Math|Rotator|BreakRotator _returnvalue))
  (bind (_x _y _z) (Math|Vector|BreakVector _returnvalue_2))
  (if (>= (Variables|Default|GetWeaponCooldown) (Variables|Default|GetWeaponSpeed))
    (bind _returnvalue_3 (Game|SpawnActorfromClass "/Game/TwinStickBP/Blueprints/GeneralProjectile.GeneralProjectile_C" (Math|Transform|MakeTransform (+ (Transformation|GetWorldLocation (Variables|Default|GetRightGun)) (Math|Vector|MakeVector (* _x _weaponoffset) (* _y _weaponoffset) _z)) (Math|Rotator|MakeRotator _roll _pitch (+ _yaw (Math|Random|RandomFloatinRange -15.0 15.0))) (Variables|Default|GetProjectileScale)) "AlwaysSpawn" 0 0))
    (Variables|/Game/TwinStickBP/Blueprints/GeneralProjectile.GeneralProjectile_C|SetDamageValue _returnvalue_3 (Variables|Default|GetWeaponStrength))
    (CallFunction|FireLeftWeapon)
    (Variables|Default|SetWeaponCooldown 0.0)))

(fn FireLeftWeapon
  (bind _returnvalue (Transformation|GetActorRotation))
  (bind _returnvalue_2 (Transformation|GetActorForwardVector))
  (bind _weaponoffset (Variables|Default|GetWeaponOffset))
  (bind (_x _y _z) (Math|Vector|BreakVector _returnvalue_2))
  (bind (_roll _pitch _yaw) (Math|Rotator|BreakRotator _returnvalue))
  (bind _returnvalue_3 (Game|SpawnActorfromClass "/Game/TwinStickBP/Blueprints/GeneralProjectile.GeneralProjectile_C" (Math|Transform|MakeTransform (+ (Transformation|GetWorldLocation (Variables|Default|GetLeftGun)) (Math|Vector|MakeVector (* _x _weaponoffset) (* _y _weaponoffset) _z)) (Math|Rotator|MakeRotator _roll _pitch (+ _yaw (Math|Random|RandomFloatinRange -3e+01 3e+01))) (Variables|Default|GetProjectileScale)) "AlwaysSpawn" 0 0))
  (Variables|/Game/TwinStickBP/Blueprints/GeneralProjectile.GeneralProjectile_C|SetDamageValue _returnvalue_3 (Variables|Default|GetWeaponStrength)))

(fn EnemySetup
  (params (Modifier :type Float%20%28single-precision%29))
  (LocalVariables|SetEnemyModifier Modifier)
  (Variables|Default|SetHealth (+ (Variables|Default|GetHealth) (LocalVariables|GetEnemyModifier)))
  (Variables|Default|SetWeaponStrength (* (LocalVariables|GetEnemyModifier) 0.2)))